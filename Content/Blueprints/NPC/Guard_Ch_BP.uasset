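; Guard NPC character Blueprint that spawns a weapon and ragdolls on death.
; BeginPlay spawns WeaponClass at an identity transform with the guard as owner, with no attachment in this graph.
; The health component's death event runs once, switching the mesh to simulated ragdoll physics and disabling capsule collision.
; The damage-taken handler is empty.
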(event `self.ReceiveBeginPlay`
  (`|SpawnActorFromClass` (`self.WeaponClass`) (`/Game/Blueprints/Shared/BLP_Library.IdentityTransform`) "AlwaysSpawn" "OverrideRootScale" self null))

(event `self.Health_Component_BC.OnDamageTaken`)

(event `self.Health_Component_BC.OnDeath`
  (`/Engine/EditorBlueprintResources/StandardMacros.DoOnce` false
    (:`Completed`
      (`PrimitiveComponent.SetCollisionProfileName` (`self.Mesh`) "Ragdoll" true)
      (`SkeletalMeshComponent.SetAllBodiesSimulatePhysics` (`self.Mesh`) true)
      (`PrimitiveComponent.WakeRigidBody` (`self.Mesh`) "None")
      (`PrimitiveComponent.SetCollisionEnabled` (`self.CapsuleComponent`) "NoCollision"))))

(fn `UserConstructionScript`)