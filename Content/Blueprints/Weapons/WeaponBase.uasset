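; Base weapon Blueprint that fires a round from its muzzle component when a fire request arrives.
; Each shot spawns a bullet actor and a fire sound, then runs a debug-drawn Visibility line trace along the muzzle's forward vector out to the weapon range.
; The hitscan trace applies point damage on a hit, credited to the owner's instigator controller, and reports a damage event for AI perception.
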(event `OnFireRequested`
  (`self.FireRound`))

(event `FireRound`
  (bind _waepon_damage (`self.waepon Damage`))
  (bind _returnvalue (`SceneComponent.K2_GetComponentLocation` (`self.MuzzlePasition`)))
  (bind _returnvalue_2 (`self.GetInstigatorController` (`self.GetOwner`)))
  (`|SpawnActorFromClass` (`self.Bullet Class`) (`SceneComponent.K2_GetComponentToWorld` (`self.MuzzlePasition`)) "AlwaysSpawn" "OverrideRootScale" null null)
  (`GameplayStatics.SpawnSoundAtLocation` "/Game/FirstPerson/Audio/FirstPersonTemplateWeaponFire02.FirstPersonTemplateWeaponFire02" _returnvalue (struct) 1.0 1.0 0.0 null null)
  (bind (_outhit _returnvalue_3) (`KismetSystemLibrary.LineTraceSingle` :`Start` _returnvalue :`End` (+ _returnvalue (* (`SceneComponent.GetForwardVector` (`self.MuzzlePasition`)) (`self.Weapon Range`))) :`TraceChannel` "TraceTypeQuery1" :`DrawDebugType` "ForDuration"))
  (if _returnvalue_3
    (bind (_bblockinghit _binitialoverlap _time _distance _location _impactpoint _normal _impactnormal _physmat _hitactor) (`GameplayStatics.BreakHitResult` _outhit))
    (`GameplayStatics.ApplyPointDamage` _hitactor _waepon_damage _impactnormal _outhit _returnvalue_2 self "/Script/Engine.DamageType")
    (`AISense_Damage.ReportDamageEvent` _hitactor _returnvalue_2 _waepon_damage _location)))

(fn `UserConstructionScript`)