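; Health_Component_BC is a shared component that tracks its owning actor's health and signals damage and death.
; On BeginPlay it fills Health to MaxHealth and binds to the owner's OnTakeAnyDamage event.
; Each positive hit broadcasts OnDamageTaken before subtracting the damage, then broadcasts OnDeath if IsDead finds Health at or below zero.
; Health is not clamped, and OnDeath fires again on further hits after death.
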(event `self.ReceiveBeginPlay`
  (set `self.Health` (`self.MaxHealth`))
  (add `Actor.OnTakeAnyDamage` (`self.GetOwner`) (delegate `OnTakeAnyDamage_Event_0`)))

(event `OnTakeAnyDamage_Event_0`
  (params (DamagedActor :type "Actor Object Reference") (Damage :type "Float (double-precision)") (DamageType :type "DamageType Object Reference") (InstigatedBy :type "Controller Object Reference") (DamageCauser :type "Actor Object Reference"))
  (if (> Damage 0.0)
    (`self.OnDamageTaken`)
    (set `self.Health` (- (`self.Health`) Damage))
    (bind _dead (`self.IsDead`))
    (if _dead
      (`self.OnDeath`))))

(fn `IsDead`
  (returns (Dead :type Boolean))
  (return (<= (`self.Health`) 0.0)))